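; BP_Waypoint is a checkpoint actor that the player collects by entering its sphere trigger.
; On BeginPlay it caches the ScaleGameMode and registers itself as a checkpoint.
; When a BP_Player that is not dead overlaps the sphere, it notifies the game mode that the checkpoint is collected, leaving all further handling to the game mode.
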(event `self.ReceiveBeginPlay`
  (bind _asscale_game_mode (cast `/Game/Blueprints/Game/ScaleGameMode` (`GameplayStatics.GetGameMode`)))
  (bind _output_get (set `self.GameMode` _asscale_game_mode))
  (`/Game/Blueprints/Game/ScaleGameMode.RegisterCheckpoint` _output_get self))

(event `self.Sphere.OnComponentBeginOverlap`
  (params (OverlappedComponent :type "PrimitiveComponent Object Reference") (OtherActor :type "Actor Object Reference") (OtherComp :type "PrimitiveComponent Object Reference") (OtherBodyIndex :type Integer) (bFromSweep :type Boolean) (SweepResult :type "HitResult Structure (by ref)"))
  (bind _asbp_player (cast `/Game/Blueprints/Characters/Player/BP_Player` OtherActor))
  (if (not (`/Game/Blueprints/Characters/Player/BP_Player.IsDeath` _asbp_player))
    (`/Game/Blueprints/Game/ScaleGameMode.CheckpointCollected` (`self.GameMode`) self)))

(fn `UserConstructionScript`)