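; Falling platform actor that drops out from under the player shortly after they step on it, then returns to its original place.
; BeginPlay stores the child component's world transform.
; When a BP_Player overlaps the Box trigger, physics simulation turns on after a short delay.
; After a further delay, ResetPhysics disables simulation and restores the saved transform.
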(event `self.ReceiveBeginPlay`
  (set `self.InitialTransform` (`SceneComponent.K2_GetComponentToWorld` (`self.Child`))))

(event `self.Box.OnComponentBeginOverlap`
  (params (OverlappedComponent :type "PrimitiveComponent Object Reference") (OtherActor :type "Actor Object Reference") (OtherComp :type "PrimitiveComponent Object Reference") (OtherBodyIndex :type Integer) (bFromSweep :type Boolean) (SweepResult :type "HitResult Structure (by ref)"))
  (cast `/Game/Blueprints/Characters/Player/BP_Player` OtherActor)
  (`KismetSystemLibrary.Delay` 1.0)
  (`PrimitiveComponent.SetSimulatePhysics` (`self.Child`) true)
  (`KismetSystemLibrary.Delay` 2.0)
  (`self.Reset Physics`))

(fn `Reset Physics`
  (`PrimitiveComponent.SetSimulatePhysics` (`self.Child`) false)
  (`SceneComponent.K2_SetWorldTransform` (`self.Child`) (`self.InitialTransform`) false false))

(fn `UserConstructionScript`)