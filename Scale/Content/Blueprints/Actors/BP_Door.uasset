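; BP_Door is a two-panel sliding door actor driven by an Interract event.
; The event reads IsOpen and instantly shifts LPanel and RPanel in opposite directions by Delta along world Y, reversing the directions when the flag is false.
; Movement uses world axes rather than the door's orientation, and this graph never changes IsOpen itself.
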(event `/Game/Blueprints/Interfaces/I_Interractable.Interract`
  (bind _l_panel (`self.L_Panel`))
  (bind _r_panel (`self.R_Panel`))
  (bind _l_panel_2 (`self.L_Panel`))
  (bind _r_panel_2 (`self.R_Panel`))
  (bind _returnvalue (`SceneComponent.K2_GetComponentToWorld` _l_panel_2))
  (bind _returnvalue_2 (`SceneComponent.K2_GetComponentToWorld` _l_panel))
  (bind _returnvalue_3 (`SceneComponent.K2_GetComponentToWorld` _r_panel))
  (bind _returnvalue_4 (`SceneComponent.K2_GetComponentToWorld` _r_panel_2))
  (if (`self.IsOpen`)
    (`SceneComponent.K2_SetWorldLocation` _l_panel (`KismetMathLibrary.MakeVector` (.x (.location _returnvalue_2)) (- (.y (.location _returnvalue_2)) (`self.Delta`)) (.z (.location _returnvalue_2))) false false)
    (`SceneComponent.K2_SetWorldLocation` _r_panel_2 (`KismetMathLibrary.MakeVector` (.x (.location _returnvalue_4)) (+ (.y (.location _returnvalue_4)) (`self.Delta`)) (.z (.location _returnvalue_4))) false false)
    (else
      (`SceneComponent.K2_SetWorldLocation` _l_panel_2 (`KismetMathLibrary.MakeVector` (.x (.location _returnvalue)) (+ (.y (.location _returnvalue)) (`self.Delta`)) (.z (.location _returnvalue))) false false)
      (`SceneComponent.K2_SetWorldLocation` _r_panel (`KismetMathLibrary.MakeVector` (.x (.location _returnvalue_3)) (- (.y (.location _returnvalue_3)) (`self.Delta`)) (.z (.location _returnvalue_3))) false false))))

(fn `UserConstructionScript`)