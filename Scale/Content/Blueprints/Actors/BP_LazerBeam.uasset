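; BP_LazerBeam is a laser beam actor that changes the player's size on contact.
; When BP_Player overlaps its capsule while the beam is active, ScaleMode decides the effect: Normal calls ScaleUp and Small calls ScaleDown.
; SwitchActivity sets the active flag and matching point light visibility, and BeginPlay uses it to start the beam switched off.
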(event `self.ReceiveBeginPlay`
  (`self.SwitchActivity` false))

(event `self.Capsule.OnComponentBeginOverlap`
  (params (OverlappedComponent :type "PrimitiveComponent Object Reference") (OtherActor :type "Actor Object Reference") (OtherComp :type "PrimitiveComponent Object Reference") (OtherBodyIndex :type Integer) (bFromSweep :type Boolean) (SweepResult :type "HitResult Structure (by ref)"))
  (bind _asbp_player (cast `/Game/Blueprints/Characters/Player/BP_Player` OtherActor))
  (if (`self.IsActive`)
    (switch `/Game/Blueprints/Game/Structures/E_PlayerSizeStates` (`self.ScaleMode`)
      (:`NewEnumerator0`
        (`/Game/Blueprints/Characters/Player/BP_Player.ScaleUp` _asbp_player))
      (:`NewEnumerator1`
        (`/Game/Blueprints/Characters/Player/BP_Player.ScaleDown` _asbp_player)))))

(fn `SwitchActivity`
  (params (SwitchOn :type Boolean))
  (bind _output_get (set `self.IsActive` SwitchOn))
  (`SceneComponent.SetVisibility` (`self.PointLight`) _output_get false))

(fn `UserConstructionScript`)