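; BP_ButtonDoor is an interactable button actor that triggers a referenced Door and lights up when used.
; The construction script creates a dynamic instance of MI_Button on its static mesh for runtime color changes.
; Its Interract event forwards the call to the Door, then sets the material's Color parameter.
; The branch condition is fixed at true, so the button always turns green and the dark red path never runs.
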(event `self.ReceiveBeginPlay`
  (`parent.ReceiveBeginPlay`))

(event `self.Interract`
  (bind _buttonmaterial (`self.ButtonMaterial`))
  (`/Game/Blueprints/Interfaces/I_Interractable.Interract` (`self.Door`))
  (if true
    (`MaterialInstanceDynamic.SetVectorParameterValue` _buttonmaterial "Color" (struct :`R` 0.065922 :`G` 1.0 :`B` 0.052083 :`A` 1.0))
    (else
      (`MaterialInstanceDynamic.SetVectorParameterValue` _buttonmaterial "Color" (struct :`R` 0.165132 :`G` 0.05448 :`B` 0.05448 :`A` 1.0)))))

(fn `UserConstructionScript`
  (`parent.UserConstructionScript`)
  (bind _returnvalue (`PrimitiveComponent.CreateDynamicMaterialInstance` (`self.StaticMesh`) 0 "/Game/Assets/Materials/Actors/MI_Button.MI_Button" "None"))
  (set `self.ButtonMaterial` _returnvalue))