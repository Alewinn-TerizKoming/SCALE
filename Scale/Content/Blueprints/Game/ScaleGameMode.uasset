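; Game mode for a player-scaling game that tracks checkpoint progress, level completion and respawning.
; Waypoints register in a map keyed by order; collection advances the current index, posts overlay notifications, and near the highest order opens the Default level after a delay.
; RespawnPlayer spawns and possesses a new player at that checkpoint, scaled down if marked Small, or at PlayerStart as fallback.
; A DoTest flag forces a test respawn on BeginPlay.
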(event `self.ReceiveBeginPlay`
  (bind _asscale_player_controller (cast `/Game/Blueprints/Game/ScalePlayerController` (`GameplayStatics.GetPlayerController` 0)))
  (bind _output_get (set `self.PlayerController` _asscale_player_controller))
  (if (`self.DoTest`)
    ;[1 0 0] TEST ONLY !
    (`self.K2_DestroyActor` (`Controller.K2_GetPawn` _output_get))
    (set `self.CurrentCheckpointIndex` (`self.Checkpoint`))
    (`self.RespawnPlayer`)))

(event `RegisterCheckpoint`
  (params (Waypoint :type "/Game/Blueprints/Actors/BP_Waypoint Object Reference"))
  (if (not (`.ReturnValue` (`BlueprintMapLibrary.Map_Find` (`self.Checkpoints`) (`/Game/Blueprints/Actors/BP_Waypoint.Order` Waypoint))))
    (`BlueprintMapLibrary.Map_Add` (`self.Checkpoints`) (`/Game/Blueprints/Actors/BP_Waypoint.Order` Waypoint) Waypoint)))

(event `CheckpointCollected`
  (params (Waypoint :type "/Game/Blueprints/Actors/BP_Waypoint Object Reference"))
  (bind _order (`/Game/Blueprints/Actors/BP_Waypoint.Order` Waypoint))
  (if (<= (`BlueprintMapLibrary.Map_Length` (`self.Checkpoints`)) 0)
    (set `self.CurrentCheckpointIndex` _order :!label _label)
    (if (>= _order (- (`BlueprintMapLibrary.Map_Length` (`self.Checkpoints`)) 2))
      (`/Game/Blueprints/UI/WG_Overlay.AddNotification` (`/Game/Blueprints/Game/ScalePlayerController.MainOverlay` (`self.PlayerController`)) "Level complete!")
      (`KismetSystemLibrary.PrintString` "TODO : level sumary")
      (`KismetSystemLibrary.Delay` 5.0)
      (set `self.DoTest` false)
      (`GameplayStatics.OpenLevelBySoftObjectPtr` "/Game/Maps/Default.Default")
      (else
        (`/Game/Blueprints/UI/WG_Overlay.AddNotification` (`/Game/Blueprints/Game/ScalePlayerController.MainOverlay` (`self.PlayerController`)) "Checkpoint reached!")))
    (elif (> _order (`self.CurrentCheckpointIndex`))
      (goto _label))))

(fn `RespawnPlayer`
  (bind _returnvalue (`GameplayStatics.GetPlayerController` 0))
  (bind (_value _returnvalue_2) (`BlueprintMapLibrary.Map_Find` (`self.Checkpoints`) (`self.CurrentCheckpointIndex`)))
  (if (> (`BlueprintMapLibrary.Map_Length` (`self.Checkpoints`)) 0)
    (if _returnvalue_2
      (bind _returnvalue_3 (`|SpawnActorFromClass` "/Game/Blueprints/Characters/Player/BP_Player.BP_Player_C" (`self.GetTransform` _value) "Undefined" "MultiplyWithRoot" null null))
      (switch `/Game/Blueprints/Game/Structures/E_PlayerSizeStates` (`/Game/Blueprints/Actors/BP_Waypoint.PlayerState` _value)
        (:`NewEnumerator0`
          _)
        (:`NewEnumerator1`
          (`/Game/Blueprints/Characters/Player/BP_Player.ScaleDown` _returnvalue_3)))
      (`Controller.Possess` _returnvalue _returnvalue_3)
      (else
        (bind _returnvalue_4 (`|SpawnActorFromClass` "/Game/Blueprints/Characters/Player/BP_Player.BP_Player_C" (`self.GetTransform` (`self.K2_FindPlayerStart` null)) "Undefined" "MultiplyWithRoot" null null :!label _label))
        (`Controller.Possess` _returnvalue _returnvalue_4)))
    (else
      (goto _label))))

(fn `UserConstructionScript`)